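; Player controller for the voxel game that owns the HUD widgets and handles menu and hotbar input.
; BeginPlay creates the main menu, debug menu, hotbar and crosshair widgets.
; The main menu toggle switches cursor, input mode and move/look blocking.
; Debug toggle and hotbar keys or scroll forward to the pawn's VoxelDebugComponent and VoxelInventoryComponent, with debug menu visibility following the component's state.
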(event EventBeginPlay
  (bind _self self)
  ;[1 1 1] Creating Main Menu Widget
  (bind _returnvalue (UserInterface|CreateWidget "/Game/MyFiles/Blueprints/UI/WBP_MainMenu.WBP_MainMenu_C" _self))
  (bind _output_get (Variables|Default|SetMainMenu _returnvalue))
  (UserInterface|Viewport|AddtoViewport _output_get 0)
  (Widget|SetVisibility _output_get "Hidden")
  ;[1 1 1] Creating Debug Menu Widget
  (bind _returnvalue_2 (UserInterface|CreateWidget "/Game/MyFiles/Blueprints/UI/WBP_DebugMenu.WBP_DebugMenu_C" _self))
  (bind _output_get_2 (Variables|Default|SetDebugMenu _returnvalue_2))
  (UserInterface|Viewport|AddtoViewport _output_get_2 0)
  (Widget|SetVisibility _output_get_2 "Collapsed")
  ;[1 1 1] Creating Hotbar Widget
  (bind _returnvalue_3 (UserInterface|CreateWidget "/Game/MyFiles/Blueprints/UI/WBP_Hotbar.WBP_Hotbar_C" _self))
  (bind _output_get_3 (Variables|Default|SetHotbar _returnvalue_3))
  (UserInterface|Viewport|AddtoViewport _output_get_3 0)
  ;[1 1 1] Creating Crosshair Widget
  (bind _returnvalue_4 (UserInterface|CreateWidget "/Game/MyFiles/Blueprints/UI/WBP_Crosshair.WBP_Crosshair_C" _self))
  (UserInterface|Viewport|AddtoViewport _returnvalue_4 0))

(event EventTick
  (params (DeltaSeconds :type Float%20%28single-precision%29)))

(event Input|ActionEvents|InputActionToggleDebugMenu
  (params (Key :type Key%20Structure :default "None"))
  (bind _returnvalue (Game|Player|GetPlayerPawn 0))
  (bind _debugmenu (Variables|Default|GetDebugMenu))
  (bind _returnvalue_2 (Actor|GetComponentbyClass _returnvalue "/Script/SmoothVoxel.VoxelDebugComponent"))
  (:Pressed
    (Class|VoxelDebugComponent|ToggleDebug _returnvalue_2)
    (if (Class|VoxelDebugComponent|IsDebugEnabled _returnvalue_2)
      (Widget|SetVisibility _debugmenu "Visible")
      (else
        (Widget|SetVisibility _debugmenu "Collapsed")))))

(event Input|ActionEvents|InputActionHotbarSlot7
  (params (Key :type Key%20Structure :default "None"))
  ;[1 1 1] Choosing hotbar slot by key 1-9
  (:Pressed
    (Class|VoxelInventoryComponent|SelectSlotbyNumber (Actor|GetComponentbyClass (Game|Player|GetPlayerPawn 0) "/Script/SmoothVoxel.VoxelInventoryComponent") 7)))

(event Input|ActionEvents|InputActionHotbarSlot8
  (params (Key :type Key%20Structure :default "None"))
  ;[1 1 1] Choosing hotbar slot by key 1-9
  (:Pressed
    (Class|VoxelInventoryComponent|SelectSlotbyNumber (Actor|GetComponentbyClass (Game|Player|GetPlayerPawn 0) "/Script/SmoothVoxel.VoxelInventoryComponent") 8)))

(event Input|ActionEvents|InputActionHotbarSlot9
  (params (Key :type Key%20Structure :default "None"))
  ;[1 1 1] Choosing hotbar slot by key 1-9
  (:Pressed
    (Class|VoxelInventoryComponent|SelectSlotbyNumber (Actor|GetComponentbyClass (Game|Player|GetPlayerPawn 0) "/Script/SmoothVoxel.VoxelInventoryComponent") 9)))

(event Input|ActionEvents|InputActionToggleMainMenu
  (params (Key :type Key%20Structure :default "None"))
  (bind _self self)
  (bind _mainmenu (Variables|Default|GetMainMenu))
  (:Pressed
    (if (Variables|Default|GetIsMenuOpen)
      (Variables|Default|SetIsMenuOpen false)
      (Widget|SetVisibility _mainmenu "Hidden")
      (Input|SetIgnoreMoveInput false)
      (Input|SetIgnoreLookInput false)
      (Variables|Default|SetbShowMouseCursor false)
      (Input|SetInputModeGameOnly _self)
      (else
        (Variables|Default|SetIsMenuOpen true)
        (Widget|SetVisibility _mainmenu "Visible")
        (Input|SetIgnoreMoveInput true)
        (Input|SetIgnoreLookInput true)
        (Variables|Default|SetbShowMouseCursor true)
        (Input|SetInputModeGameandUI _self _mainmenu "DoNotLock" false)))))

(event Input|ActionEvents|InputActionHotbarSlot1
  (params (Key :type Key%20Structure :default "None"))
  ;[1 1 1] Choosing hotbar slot by key 1-9
  (:Pressed
    (Class|VoxelInventoryComponent|SelectSlotbyNumber (Actor|GetComponentbyClass (Game|Player|GetPlayerPawn 0) "/Script/SmoothVoxel.VoxelInventoryComponent") 1)))

(event Input|ActionEvents|InputActionHotbarSlot2
  (params (Key :type Key%20Structure :default "None"))
  ;[1 1 1] Choosing hotbar slot by key 1-9
  (:Pressed
    (Class|VoxelInventoryComponent|SelectSlotbyNumber (Actor|GetComponentbyClass (Game|Player|GetPlayerPawn 0) "/Script/SmoothVoxel.VoxelInventoryComponent") 2)))

(event Input|ActionEvents|InputActionHotbarSlot3
  (params (Key :type Key%20Structure :default "None"))
  ;[1 1 1] Choosing hotbar slot by key 1-9
  (:Pressed
    (Class|VoxelInventoryComponent|SelectSlotbyNumber (Actor|GetComponentbyClass (Game|Player|GetPlayerPawn 0) "/Script/SmoothVoxel.VoxelInventoryComponent") 3)))

(event Input|ActionEvents|InputActionHotbarSlot4
  (params (Key :type Key%20Structure :default "None"))
  ;[1 1 1] Choosing hotbar slot by key 1-9
  (:Pressed
    (Class|VoxelInventoryComponent|SelectSlotbyNumber (Actor|GetComponentbyClass (Game|Player|GetPlayerPawn 0) "/Script/SmoothVoxel.VoxelInventoryComponent") 4)))

(event Input|ActionEvents|InputActionHotbarSlot5
  (params (Key :type Key%20Structure :default "None"))
  ;[1 1 1] Choosing hotbar slot by key 1-9
  (:Pressed
    (Class|VoxelInventoryComponent|SelectSlotbyNumber (Actor|GetComponentbyClass (Game|Player|GetPlayerPawn 0) "/Script/SmoothVoxel.VoxelInventoryComponent") 5)))

(event Input|ActionEvents|InputActionHotbarSlot6
  (params (Key :type Key%20Structure :default "None"))
  ;[1 1 1] Choosing hotbar slot by key 1-9
  (:Pressed
    (Class|VoxelInventoryComponent|SelectSlotbyNumber (Actor|GetComponentbyClass (Game|Player|GetPlayerPawn 0) "/Script/SmoothVoxel.VoxelInventoryComponent") 6)))

(event Input|AxisEvents|InputAxisHotbarScroll
  (params (AxisValue :type Float%20%28single-precision%29))
  (bind _returnvalue (Game|Player|GetPlayerPawn 0))
  (bind _returnvalue_2 (Actor|GetComponentbyClass _returnvalue "/Script/SmoothVoxel.VoxelInventoryComponent"))
  (if (< AxisValue 0.0)
    (Class|VoxelInventoryComponent|SelectNextSlot _returnvalue_2)
    (elif (> AxisValue 0.0)
      (Class|VoxelInventoryComponent|SelectPreviousSlot _returnvalue_2))))

(fn ConstructionScript)